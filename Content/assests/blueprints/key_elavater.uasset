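; Keycard-locked elevator actor that moves its static mesh between a start and end point.
; A trigger overlap checks the ThirdPersonCharacter's Keycards array and enables player input only when the entry at KeycardValue is true; leaving the trigger disables it.
; Pressing E then plays a timeline that lerps the mesh's relative location from Startpoint to Endpoint.
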(event `self.trigger.OnComponentBeginOverlap`
  (params (OverlappedComponent :type "PrimitiveComponent Object Reference") (OtherActor :type "Actor Object Reference") (OtherComp :type "PrimitiveComponent Object Reference") (OtherBodyIndex :type Integer) (bFromSweep :type Boolean) (SweepResult :type "HitResult Structure (by ref)"))
  (bind _asthird_person_character (cast `/Game/ThirdPersonBP/Blueprints/ThirdPersonCharacter` OtherActor))
  (for (_array_element _array_index) (`/Game/ThirdPersonBP/Blueprints/ThirdPersonCharacter.keycards` _asthird_person_character)
    (if (and _array_element (== _array_index (`self.keycard_value`)))
      (`self.EnableInput` (`GameplayStatics.GetPlayerController` 0)))))

(event `self.trigger.OnComponentEndOverlap`
  (params (OverlappedComponent :type "PrimitiveComponent Object Reference") (OtherActor :type "Actor Object Reference") (OtherComp :type "PrimitiveComponent Object Reference") (OtherBodyIndex :type Integer))
  (cast `/Game/ThirdPersonBP/Blueprints/ThirdPersonCharacter` OtherActor)
  (`self.DisableInput` (`GameplayStatics.GetPlayerController` 0)))

(event `Key|E`
  (params (Key :type "Key Structure"))
  (:`Pressed`
    (bind (_direction _newtrack_0) (`Timeline|Timeline_0`)
      (:`Update`
        (`SceneComponent.K2_SetRelativeLocation` (`self.StaticMesh`) (`KismetMathLibrary.VLerp` (`self.startpoint`) (`self.endpoint`) _newtrack_0) false false)))))

(fn `UserConstructionScript`)